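; BP_Wand is a wand Blueprint that plays the visual effect for the Periculum spell.
; On BeginPlay it binds an event to the PericulumFire dispatcher.
; When fired, the event spawns the NS_Periculum Niagara system slightly ahead of the WandEnd socket on WandMesh, using the socket's rotation.
; The effect is deliberately left unattached so it stays at the firing location instead of following the wand.
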(event `self.ReceiveBeginPlay`
  (add `self.PericulumFire` (delegate `PericulumFire_Event_0`)))

(event `PericulumFire_Event_0`
  (bind _rotation (.rotation (`SceneComponent.GetSocketTransform` (`self.WandMesh`) "WandEnd" "RTS_World")))
  ;[1 1 1] We don't want to attach it as we want it to be from the loc not following the wand
  (bind _returnvalue (`NiagaraFunctionLibrary.SpawnSystemAtLocation` "/Game/Effects/Periculum/NS_Periculum.NS_Periculum" (+ (.location (`SceneComponent.GetSocketTransform` (`self.WandMesh`) "WandEnd" "RTS_World")) (* (`KismetMathLibrary.Conv_RotatorToVector` _rotation) 5.0)) _rotation)))

(fn `UserConstructionScript`)