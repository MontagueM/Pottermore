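; Projectile Blueprint that reacts to sphere collisions, including hits on Protego wall blocks.
; On hit, it sets IsProtegoWall if the other actor is a BP_BlockMesh, then forwards the hit data and flag to Hit.
; Every hit also spawns the scaled NS_ProtegoHit Niagara effect at the impact point, oriented by the impact normal rotated around Y, and prints a debug string.
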(event `self.Sphere.OnComponentHit`
  (params (HitComponent :type "PrimitiveComponent Object Reference") (OtherActor :type "Actor Object Reference") (OtherComp :type "PrimitiveComponent Object Reference") (NormalImpulse :type "Vector Structure") (Hit :type "HitResult Structure (by ref)"))
  (cast `/Game/Effects/Protego/BP_BlockMesh` OtherActor
    (:`then`
      (set `self.bIsProtegoWall` true))
    (:`CastFailed`
      _))
  (`self.Hit` HitComponent OtherActor OtherComp NormalImpulse Hit (`self.bIsProtegoWall`))
  (`self.SpawnBlockNiagaraEffect` Hit)
  (`KismetSystemLibrary.PrintString` "Hello"))

(event `SpawnBlockNiagaraEffect`
  (params (Result :type "HitResult Structure"))
  (bind (_bblockinghit _binitialoverlap _time _distance _location _impactpoint _normal _impactnormal) (`GameplayStatics.BreakHitResult` Result))
  (`NiagaraFunctionLibrary.SpawnSystemAtLocation` "/Game/Effects/Protego/NS_ProtegoHit.NS_ProtegoHit" _location (`KismetMathLibrary.Conv_VectorToRotator` (`KismetMathLibrary.RotateAngleAxis` _impactnormal 90.0 (0.0 1.0 0.0))) (10.0 10.0 10.0)))

(fn `UserConstructionScript`)